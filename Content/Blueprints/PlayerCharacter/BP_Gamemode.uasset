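; Game mode that runs the in-game clock and triggers timed player deaths and a red lighting change.
; Tick uses a Delay to step Time while the player is alive, unpaused and out of menus, deriving Hours and Seconds from it.
; When Seconds reaches 59 on a listed death time, it marks Dead and calls the HUD's death listener.
; From a set time onward, it turns the SkyLight and every BP_Light red.
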(event EventBeginPlay
  (bind _time (Variables|Timer|GetTime))
  (Variables|Timer|SetHours (Math|Float|Floor (/ _time 6e+01)))
  (Variables|Timer|SetSeconds (Math|Float|Truncate (Math|Float|%(Float) _time 6e+01)))
  (bind _asbp_hud (Utilities|Casting|CastToBP_HUD (HUD|GetHUD (Game|GetPlayerController 0))))
  (Variables|Default|SetHUD _asbp_hud)
  (bind _asbp_player_character (Utilities|Casting|CastToBP_PlayerCharacter (Game|GetPlayerCharacter 0)))
  (Variables|Default|SetPlayerReference _asbp_player_character))

(event EventTick
  (params (DeltaSeconds :type Float%20%28single-precision%29))
  (bind _playerreference (Variables|Default|GetPlayerReference))
  (if (not (Math|Boolean|ORBoolean (Variables|Default|GetDead) (Variables|/Game/Blueprints/PlayerCharacter/BP_PlayerCharacter.BP_PlayerCharacter_C|GetbIsPaused? _playerreference) (Variables|/Game/Blueprints/PlayerCharacter/BP_PlayerCharacter.BP_PlayerCharacter_C|GetbIsInMenu? _playerreference)))
    (Utilities|FlowControl|Delay (Variables|Timer|GetDelayTime))
    (Utilities|FlowControl|Sequence
      (:then_0
        (if (== (Variables|Timer|GetSeconds) 59)
          (if (Utilities|Array|ContainsItem (Variables|Timer|GetDeathTimes) (Variables|Timer|GetTime))
            (Variables|Default|SetDead true)
            (Default|CallDeathEventListener (Variables|Default|GetHUD) "NewEnumerator0"))))
      (:then_1
        (Variables|Timer|SetTime (+ (Variables|Timer|GetTime) 1.0))
        (Variables|Timer|SetHours (Math|Float|Floor (/ (Variables|Timer|GetTime) 6e+01)))
        (Variables|Timer|SetSeconds (Math|Float|Truncate (Math|Float|%(Float) (Variables|Timer|GetTime) 6e+01))))
      (:then_2
        (if (not (Variables|Default|GetbAreLightsRed?))
          (if (>= (Variables|Timer|GetTime) 6.6e+02)
            (bind _returnvalue (Actor|GetActorOfClass "/Script/Engine.SkyLight"))
            (Rendering|Components|Light|SetLightColor (Variables|/Script/Engine.SkyLight|GetLightComponent _returnvalue) "(R=1.000000,G=0.000000,B=0.000000,A=1.000000)")
            (bind _outactors (Actor|GetAllActorsOfClass "/Game/Blueprints/OfficeDecorations/BP_Light.BP_Light_C"))
            (for _array_element _outactors
              (Default|EnableRedLights _array_element)
              (Variables|Default|SetbAreLightsRed? true))))))))

(fn ConstructionScript)