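; Base contract actor: a paper document that tears itself in half one second after BeginPlay.
; SetReferences stores the contract information and caches the player character and HUD.
; DestroyContract runs once, swapping the intact paper mesh for two physics-simulated halves.
; Randomly scaled, opposite impulses in the paper's local X axis, applied at an offset along its forward vector, fling the halves apart.
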(event EventBeginPlay
  (Utilities|FlowControl|Delay 1.0)
  (CallFunction|DestroyContract))

(fn ConstructionScript)

(fn SetReferences
  (params (Information :type Text))
  (Variables|Default|SetInformation Information)
  (bind _asbp_player_character (Utilities|Casting|CastToBP_PlayerCharacter (Game|GetPlayerCharacter 0)))
  (Variables|Default|SetPlayerReference _asbp_player_character)
  (bind _asbp_hud (Utilities|Casting|CastToBP_HUD (HUD|GetHUD (Game|GetPlayerController 0))))
  (Variables|Default|SetHUDReference _asbp_hud))

(fn DestroyContract
  (bind _returnvalue (Math|Random|RandomFloatinRange 1.0 1.5))
  (bind _papermesh (Variables|Default|GetPaperMesh))
  (bind _rightside (Variables|Default|GetRightSide))
  (bind _tear_strength (Variables|Default|GetTear%20Strength))
  (bind _papermesh_2 (Variables|Default|GetPaperMesh))
  (bind _returnvalue_2 (Transformation|GetWorldLocation _papermesh_2))
  (bind _returnvalue_3 (Transformation|GetWorldRotation _papermesh_2))
  (bind _returnvalue_4 (* _tear_strength _returnvalue))
  (bind _returnvalue_5 (Math|Vector|GetForwardVector _returnvalue_3))
  (bind _returnvalue_6 (* _returnvalue_5 1e+02))
  (bind _returnvalue_7 (+ _returnvalue_2 _returnvalue_6))
  (if (not (Variables|Default|GetbContractDestroyed?))
    (Variables|Default|SetbContractDestroyed? true)
    (Physics|SetSimulatePhysics _papermesh false)
    (Physics|SetSimulatePhysics _rightside true)
    (Rendering|SetVisibility _papermesh false false)
    (Rendering|SetVisibility _rightside true false)
    (Physics|AddImpulseatLocation _rightside (Math|Vector|RotateVector (* "1.000000,0.000000,0.000000" _returnvalue_4) _returnvalue_3) _returnvalue_7 "None")
    (Physics|AddImpulseatLocation (Variables|Default|GetLeftSide) (Math|Vector|RotateVector (* "-1.000000, 0,0.000000" _returnvalue_4) _returnvalue_3) _returnvalue_7 "None")))