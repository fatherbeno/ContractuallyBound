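; A contract actor that trades restored player jumping for hostile chairs, reading "JUMPING IS PROHIBITED BUT CHAIRS ARE PEACEFUL".
; On BeginPlay it passes that text to SetReferences.
; Triggering it enables jumping on the player reference, flags chairs as aggressive on the game mode, then destroys the contract.
; ContractInformation forwards the look-at and destroyed states to SetContractInformation.
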(event EventBeginPlay
  (CallFunction|SetReferences "JUMPING IS PROHIBITED BUT CHAIRS ARE PEACEFUL"))

(event EventTriggerContract
  (Variables|/Game/Blueprints/PlayerCharacter/BP_PlayerCharacter.BP_PlayerCharacter_C|SetbCanJump? (Variables|Default|GetPlayerReference) true)
  (Variables|/Game/Blueprints/PlayerCharacter/BP_Gamemode.BP_Gamemode_C|SetbAreChairsAgro? (Variables|Default|GetGamemodeReference) true)
  (CallFunction|DestroyContract))

(event EventContractInformation
  (params (bIsLookingAtContract? :type Boolean))
  (Utilities|SetContractInformation (Variables|Default|GetbContractDestroyed?) bIsLookingAtContract?))

(fn ConstructionScript
  (|CallParentFunction))