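; Contract Blueprint that trades opened vents for a lava floor when triggered.
; On BeginPlay it registers its current-state text (vents locked, floor not lava) and caches every BP_Vent in the level.
; Triggering sets FloorIsLava on the player, enables physics on each vent mesh with a sound at its location, then destroys the contract.
; Look-at events pass the destroyed and looked-at state to SetContractInformation.
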(event EventBeginPlay
  (CallFunction|SetReferences "VENTS ARE LOCKED BUT FLOOR IS NOT LAVA")
  (bind _outactors (Actor|GetAllActorsOfClass "/Game/Blueprints/OfficeDecorations/BP_Vent.BP_Vent_C"))
  (Variables|Default|SetVents _outactors))

(event EventTriggerContract
  (Variables|/Game/Blueprints/PlayerCharacter/BP_PlayerCharacter.BP_PlayerCharacter_C|SetbFloorIsLava? (Variables|Default|GetPlayerReference) true)
  (for _array_element (Variables|Default|GetVents)
    (Physics|SetSimulatePhysics (Variables|/Game/Blueprints/OfficeDecorations/BP_Vent.BP_Vent_C|GetVent _array_element) true)
    (Audio|PlaySoundatLocation "/Game/Audio/SoundCues/Vent_Cue.Vent_Cue" (Transformation|GetActorLocation _array_element) "0, 0, 0" 1.0 1.0 0.0 0 0 0))
  (CallFunction|DestroyContract))

(event EventContractInformation
  (params (bIsLookingAtContract? :type Boolean))
  (Utilities|SetContractInformation (Variables|Default|GetbContractDestroyed?) bIsLookingAtContract?))

(fn ConstructionScript
  (|CallParentFunction))