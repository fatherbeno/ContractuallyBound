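; Contract actor that, when triggered, changes the gamemode's delay time and desk drawer rule, then destroys itself.
; On BeginPlay it registers its text through SetReferences, and ContractInformation passes look-at and destroyed state to the contract display logic.
; Its text says drawers cannot open and the floor is not lava, yet triggering sets CanOpenDeskDrawers true and the FloorIsLava setter is unconnected.
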(event EventBeginPlay
  (CallFunction|SetReferences "CANNOT OPEN DESK DRAWERS BUT THE FLOOR IS NOT LAVA"))

(event EventTriggerContract
  (Variables|/Game/Blueprints/PlayerCharacter/BP_Gamemode.BP_Gamemode_C|SetDelayTime (Variables|Default|GetGamemodeReference) 0.5)
  (Variables|/Game/Blueprints/PlayerCharacter/BP_Gamemode.BP_Gamemode_C|SetbCanOpenDeskDrawers? (Variables|Default|GetGamemodeReference) true)
  (CallFunction|DestroyContract))

(event EventContractInformation
  (params (bIsLookingAtContract? :type Boolean))
  (Utilities|SetContractInformation (Variables|Default|GetbContractDestroyed?) bIsLookingAtContract?))

(fn ConstructionScript
  (|CallParentFunction))