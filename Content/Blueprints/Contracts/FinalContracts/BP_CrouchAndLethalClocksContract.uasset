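; Contract actor for a rule trade-off, labelled "CROUCHING IS BANNED BUT CLOCKS ARE NOT LETHAL".
; On BeginPlay it passes that clause text to the inherited SetReferences.
; Triggering it lifts both halves of the clause by re-enabling crouch on the player and clock deaths on the game mode, then destroys the contract.
; ContractInformation forwards the destroyed and looked-at states to SetContractInformation.
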(event EventBeginPlay
  (CallFunction|SetReferences "CROUCHING IS BANNED BUT CLOCKS ARE NOT LETHAL"))

(event EventTriggerContract
  (Variables|/Game/Blueprints/PlayerCharacter/BP_PlayerCharacter.BP_PlayerCharacter_C|SetbCanCrouch? (Variables|Default|GetPlayerReference) true)
  (Variables|/Game/Blueprints/PlayerCharacter/BP_Gamemode.BP_Gamemode_C|SetbCanDieFromClock? (Variables|Default|GetGamemodeReference) true)
  (CallFunction|DestroyContract))

(event EventContractInformation
  (params (bIsLookingAtContract? :type Boolean))
  (Utilities|SetContractInformation (Variables|Default|GetbContractDestroyed?) bIsLookingAtContract?))

(fn ConstructionScript
  (|CallParentFunction))