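; Contract Blueprint for the rule "Cabinets are locked but clocks obey gravity", which changes cabinet and clock behavior when triggered.
; On BeginPlay it registers its contract text and caches every BP_Clock in the level.
; Triggering it allows cabinet opening through the game mode, removes each clock's gravity event listener, then destroys the contract.
; A separate event passes the destroyed and looked-at states to the contract information setter.
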(event EventBeginPlay
  (CallFunction|SetReferences "CABINETS ARE LOCKED BUT CLOCKS OBEY GRAVITY")
  (bind _outactors (Actor|GetAllActorsOfClass "/Game/Blueprints/OfficeDecorations/BP_Clock.BP_Clock_C"))
  (Variables|Default|SetClocks _outactors))

(event EventTriggerContract
  (Variables|/Game/Blueprints/PlayerCharacter/BP_Gamemode.BP_Gamemode_C|SetbCanOpenCabinets? (Variables|Default|GetGamemodeReference) true)
  (for _array_element (Variables|Default|GetClocks)
    (Default|CallRemoveGravityEventListener _array_element))
  (CallFunction|DestroyContract))

(event EventContractInformation
  (params (bIsLookingAtContract? :type Boolean))
  (Utilities|SetContractInformation (Variables|Default|GetbContractDestroyed?) bIsLookingAtContract?))

(fn ConstructionScript
  (|CallParentFunction))