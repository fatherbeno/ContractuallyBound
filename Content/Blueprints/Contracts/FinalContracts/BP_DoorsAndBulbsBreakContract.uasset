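; A contract Blueprint that, when triggered, turns off every BP_Light in the level and then destroys itself through DestroyContract.
; It caches the lights at BeginPlay and forwards look-at and destroyed state to SetContractInformation.
; Despite the doors in its name, it contains no door logic, and SetReferences still receives the placeholder string "EXAMPLE".
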(event EventBeginPlay
  (CallFunction|SetReferences "EXAMPLE")
  (bind _outactors (Actor|GetAllActorsOfClass "/Game/Blueprints/OfficeDecorations/BP_Light.BP_Light_C"))
  (Variables|Default|SetLights _outactors))

(event EventTriggerContract
  (for _array_element (Variables|Default|GetLights)
    (Default|CallTurnOffLight _array_element))
  (CallFunction|DestroyContract))

(event EventContractInformation
  (params (bIsLookingAtContract? :type Boolean))
  (Utilities|SetContractInformation (Variables|Default|GetbContractDestroyed?) bIsLookingAtContract?))

(fn ConstructionScript
  (|CallParentFunction))