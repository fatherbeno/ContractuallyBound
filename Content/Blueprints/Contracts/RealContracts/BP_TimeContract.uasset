(event Custom|AddDeathTime
  (Utilities|Array|Add (Variables|/Game/Blueprints/PlayerCharacter/BP_Gamemode.BP_Gamemode_C|GetDeathTimes (Variables|Default|GetGamemodeReference)) (- (Variables|Default|GetDeathTime) 1.0)))

(event Custom|RemoveDeathTime
  (Utilities|Array|RemoveItem (Variables|/Game/Blueprints/PlayerCharacter/BP_Gamemode.BP_Gamemode_C|GetDeathTimes (Variables|Default|GetGamemodeReference)) (- (Variables|Default|GetDeathTime) 1.0)))

(event EventBeginPlay
  (bind _deathtime (Variables|Default|GetDeathTime))
  (CallFunction|SetReferences (Utilities|Text|ToText(String) (Utilities|String|Append "YOU WILL DIE AT " (Utilities|String|Append (Utilities|String|ToString(Integer) (Math|Float|Floor (/ _deathtime 6e+01))) ":" (Utilities|String|Right (Utilities|String|Append "0" (Utilities|String|ToString(Integer) (Math|Float|Truncate (Math|Float|%(Float) _deathtime 6e+01)))) 2)) (select (>= (Variables|Default|GetDeathTime) 7.2e+02) "AM" "PM"))))
  (CallFunction|AddDeathTime))

(event EventContractInformation
  (params (bIsLookingAtContract? :type Boolean))
  (Utilities|SetContractInformation (Variables|Default|GetbContractDestroyed?) bIsLookingAtContract?))

(event EventTriggerContract
  (CallFunction|RemoveDeathTime)
  (CallFunction|DestroyContract))

(fn ConstructionScript
  (|CallParentFunction))