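; A contract actor that, when triggered, grants the player crouching and turns off the gravity event listening of the level's clocks.
; On BeginPlay it sets up its references and caches every BP_Clock in the level.
; Triggering enables CanCrouch on the player, calls each clock to remove its gravity event listener, then destroys the contract.
; A separate event forwards look-at and destroyed state to the contract information display.
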(event EventBeginPlay
  (CallFunction|SetReferences)
  (bind _outactors (Actor|GetAllActorsOfClass "/Game/Blueprints/OfficeDecorations/BP_Clock.BP_Clock_C"))
  (Variables|Default|SetClocks _outactors))

(event EventTriggerContract
  (Variables|/Game/Blueprints/PlayerCharacter/BP_PlayerCharacter.BP_PlayerCharacter_C|SetbCanCrouch? (Variables|Default|GetPlayerReference) true)
  (for _array_element (Variables|Default|GetClocks)
    (Default|CallRemoveGravityEventListener _array_element))
  (CallFunction|DestroyContract))

(event EventContractInformation
  (params (bIsLookingAtContract? :type Boolean))
  (Utilities|SetContractInformation (Variables|Default|GetbContractDestroyed?) bIsLookingAtContract?))

(fn ConstructionScript
  (|CallParentFunction))