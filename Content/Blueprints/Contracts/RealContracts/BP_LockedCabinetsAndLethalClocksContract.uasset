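; Contract actor that, when triggered, makes clocks lethal and affects cabinet access through game mode flags.
; Triggering sets both CanDieFromClock and CanOpenCabinets to true, despite the "LockedCabinets" name, then destroys the contract.
; BeginPlay sets up references with an "EXAMPLE" placeholder string, and ContractInformation forwards look-at and destroyed state to SetContractInformation.
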(event EventBeginPlay
  (CallFunction|SetReferences "EXAMPLE"))

(event EventTriggerContract
  (bind _gamemodereference (Variables|Default|GetGamemodeReference))
  (Variables|/Game/Blueprints/PlayerCharacter/BP_Gamemode.BP_Gamemode_C|SetbCanDieFromClock? _gamemodereference true)
  (Variables|/Game/Blueprints/PlayerCharacter/BP_Gamemode.BP_Gamemode_C|SetbCanOpenCabinets? _gamemodereference true)
  (CallFunction|DestroyContract))

(event EventContractInformation
  (params (bIsLookingAtContract? :type Boolean))
  (Utilities|SetContractInformation (Variables|Default|GetbContractDestroyed?) bIsLookingAtContract?))

(fn ConstructionScript
  (|CallParentFunction))