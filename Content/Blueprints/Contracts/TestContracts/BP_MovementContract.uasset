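; Test contract actor that grants the player permission to walk.
; On BeginPlay it sets its references under a contract title and disables the player's CanWalk flag.
; TriggerContract re-enables walking and destroys the contract, and ContractInformation passes the destroyed state to SetContractInformation.
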(event EventBeginPlay
  (CallFunction|SetReferences "CONTRACT: Permission to Walk")
  (Variables|/Game/Blueprints/PlayerCharacter/BP_PlayerCharacter.BP_PlayerCharacter_C|SetbCanWalk? (Variables|Default|GetPlayerReference) false))

(event EventTriggerContract
  (Variables|/Game/Blueprints/PlayerCharacter/BP_PlayerCharacter.BP_PlayerCharacter_C|SetbCanWalk? (Variables|Default|GetPlayerReference) true)
  (CallFunction|DestroyContract))

(event EventContractInformation
  (Utilities|SetContractInformation (Variables|Default|GetbContractDestroyed?)))

(fn ConstructionScript
  (|CallParentFunction))