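; BP_Light is an office decoration light, made of a SpotLight and a light mesh, that can switch off or turn red.
; On BeginPlay it binds its OFF event to TurnOffLight, and OFF sets both components' visibility to the inverse of the Malfunction flag.
; EnableRedLights tints the spotlight red and swaps the mesh to a red light material.
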(event Custom|OFF
  (Rendering|SetVisibility (Variables|Default|GetSpotLight) (not (Variables|Default|GetbMalfunction?)) false))

(event Custom|EnableRedLights
  (Rendering|Components|Light|SetLightColor (Variables|Default|GetSpotLight) "(R=1.000000,G=0.000000,B=0.000000,A=1.000000)" true)
  (Rendering|Material|SetMaterial (Variables|Default|GetLightMesh) 0 "/Game/Materials/RedLightMaterial_Inst.RedLightMaterial_Inst"))

(event EventBeginPlay
  (EventDispatchers|BindEventtoTurnOffLight (delegate Custom|OFF)))

(fn ConstructionScript)