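; BP_Clock is an office decoration that displays the in-game time on four separate digit texts.
; On BeginPlay it caches BP_Gamemode, the source of the time values.
; Tick, throttled by a short Delay, zero-pads the game mode's Hours and Seconds with string operations and splits them into the digits.
; The second pair reads the Seconds variable, with no separate minutes value used.
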(event EventBeginPlay
  (bind _asbp_gamemode (Utilities|Casting|CastToBP_Gamemode (Game|GetGameMode)))
  (Variables|Default|SetGamemodeReference _asbp_gamemode))

(event EventTick
  (params (DeltaSeconds :type Float%20%28single-precision%29))
  (bind _gamemodereference (Variables|Default|GetGamemodeReference))
  (bind _hours (Variables|/Game/Blueprints/PlayerCharacter/BP_Gamemode.BP_Gamemode_C|GetHours _gamemodereference))
  (bind _seconds (Variables|/Game/Blueprints/PlayerCharacter/BP_Gamemode.BP_Gamemode_C|GetSeconds _gamemodereference))
  (bind _returnvalue (Utilities|String|ToString(Integer) _hours))
  (bind _returnvalue_2 (Utilities|String|ToString(Integer) _seconds))
  (bind _returnvalue_3 (Utilities|String|Append "0" _returnvalue))
  (bind _returnvalue_4 (Utilities|String|Append "0" _returnvalue_2))
  (bind _returnvalue_5 (Utilities|String|Right _returnvalue_3 2))
  (bind _returnvalue_6 (Utilities|String|Right _returnvalue_4 2))
  (Utilities|FlowControl|Delay 0.1)
  (Rendering|Components|TextRender|SetText (Variables|Default|GetDigit1Text) (Utilities|Text|ToText(String) (Utilities|String|Left _returnvalue_5 1)))
  (Rendering|Components|TextRender|SetText (Variables|Default|GetDigit2Text) (Utilities|Text|ToText(String) (Utilities|String|Right _returnvalue_5 1)))
  (Rendering|Components|TextRender|SetText (Variables|Default|GetDigit3Text) (Utilities|Text|ToText(String) (Utilities|String|Left _returnvalue_6 1)))
  (Rendering|Components|TextRender|SetText (Variables|Default|GetDigit4Text) (Utilities|Text|ToText(String) (Utilities|String|Right _returnvalue_6 1))))

(fn ConstructionScript)