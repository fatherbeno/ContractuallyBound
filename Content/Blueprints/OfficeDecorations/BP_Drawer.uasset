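; BP_Drawer is an office decoration drawer that slides open or closed when it receives the OfficeInteract event.
; Each interaction plays the matching open or close sound at the frame, then a timeline lerps the drawer along its relative Y axis from its current position.
; A DoOnce gate blocks re-triggering until the timeline finishes, when ResetDoOnce flips AmOpen and re-arms it.
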(event Custom|ResetDoOnce
  (Variables|Default|SetbAmOpen? (not (Variables|Default|GetbAmOpen?)))
  (Utilities|FlowControl|DoOnce false) ; enters at Reset
)

(event EventOfficeInteract
  (Utilities|FlowControl|DoOnce false
    (:Completed
      (Variables|Default|SetRelative%20Location (Variables|/Script/Engine.SceneComponent|GetRelativeLocation (Variables|Default|GetDrawer)))
      (Audio|PlaySoundatLocation (select (Variables|Default|GetbAmOpen?) "/Game/Audio/SoundCues/DrawerClose_Cue.DrawerClose_Cue" "/Game/Audio/SoundCues/draweropen_Cue.DrawerOpen_Cue") (Transformation|GetWorldLocation (Variables|Default|GetDrawerFrame)) "0, 0, 0" 1.0 1.0 0.0 0 0 0)
      (bind _toone (Timeline|ActivateDrawerTimeline PlayFromStart)
        (:Update
          (Transformation|SetRelativeLocation (Variables|Default|GetDrawer) (Math|Vector|Lerp(Vector) (Variables|Default|GetRelative%20Location) (select (Variables|Default|GetbAmOpen?) (- (Variables|Default|GetRelative%20Location) "0,100.000000, 0") (+ (Variables|Default|GetRelative%20Location) "0,100.000000, 0")) _toone) false false))
        (:Finished
          (CallFunction|ResetDoOnce))))))

(fn ConstructionScript)